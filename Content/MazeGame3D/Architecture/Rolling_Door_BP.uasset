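; Rolling door actor for the 3D maze game that slides and rotates open or closed when interacted with.
; A single timeline drives the mesh's X position and pitch, playing forward to open and in reverse to close, and flips the open flag when finished.
; Interact sets the play rate from separate open and close durations.
; Ending overlap with the box also reverses the timeline.
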(event OnComponentEndOverlap(Box)
  (params (OverlappedComponent :type Primitive%20Component%20Object%20Reference) (OtherActor :type Actor%20Object%20Reference) (OtherComp :type Primitive%20Component%20Object%20Reference) (OtherBodyIndex :type Integer))
  (bind (_direction _door_track _rotation_track) (Timeline|OpenDoorT Reverse)
    (:Update
      (Transformation|SetRelativeLocationAndRotation (Variables|Default|GetDoorStaticMesh) (Math|Vector|MakeVector (Math|Float|Lerp (Variables|Default|GetClosePosition) (Variables|Default|GetOpenPosition) _door_track) 0.0 75.0) (Math|Rotator|MakeRotator 0.0 (Math|Float|Lerp (Variables|Default|GetDoor_Rotation_Finish) (Variables|Default|GetDoor_Rotation_Start) _rotation_track) 0.0) false false))
    (:Finished
      (Variables|Default|SetisOpen? (not (Variables|Default|GetisOpen?))))))

(event Custom|OpenDoor
  (bind (_direction _door_track _rotation_track) (Timeline|OpenDoorT Play)
    (:Update
      (Transformation|SetRelativeLocationAndRotation (Variables|Default|GetDoorStaticMesh) (Math|Vector|MakeVector (Math|Float|Lerp (Variables|Default|GetClosePosition) (Variables|Default|GetOpenPosition) _door_track) 0.0 75.0) (Math|Rotator|MakeRotator 0.0 (Math|Float|Lerp (Variables|Default|GetDoor_Rotation_Finish) (Variables|Default|GetDoor_Rotation_Start) _rotation_track) 0.0) false false))
    (:Finished
      (Variables|Default|SetisOpen? (not (Variables|Default|GetisOpen?))))))

(event Custom|CloseDoor
  (bind (_direction _door_track _rotation_track) (Timeline|OpenDoorT Reverse)
    (:Update
      (Transformation|SetRelativeLocationAndRotation (Variables|Default|GetDoorStaticMesh) (Math|Vector|MakeVector (Math|Float|Lerp (Variables|Default|GetClosePosition) (Variables|Default|GetOpenPosition) _door_track) 0.0 75.0) (Math|Rotator|MakeRotator 0.0 (Math|Float|Lerp (Variables|Default|GetDoor_Rotation_Finish) (Variables|Default|GetDoor_Rotation_Start) _rotation_track) 0.0) false false))
    (:Finished
      (Variables|Default|SetisOpen? (not (Variables|Default|GetisOpen?))))))

(fn ConstructionScript)

(fn Interact
  (params (Interactor :type Character%20Object%20Reference))
  (bind _opendoort (Variables|Default|GetOpenDoorT))
  (if (not (Variables|Default|GetisOpen?))
    (Components|Timeline|SetPlayRate _opendoort (/ 1.0 (Variables|Default|GetOpenTime%28sec%29)))
    (CallFunction|OpenDoor)
    (else
      (Components|Timeline|SetPlayRate _opendoort (/ 1.0 (Variables|Default|GetCloseTime%28sec%29)))
      (CallFunction|CloseDoor)))
  (return false))