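; Interactable hinged door for the maze game that swings its static mesh in yaw between closed and open positions.
; Interact checks IsOpen, sets the timeline play rate from the open or close duration, then plays or reverses it.
; The OpenDoorT timeline drives the rotation lerp and flips IsOpen whenever it finishes.
; Ending overlap with the Box also reverses the timeline, without resetting the play rate.
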(event OnComponentEndOverlap(Box)
  (params (OverlappedComponent :type Primitive%20Component%20Object%20Reference) (OtherActor :type Actor%20Object%20Reference) (OtherComp :type Primitive%20Component%20Object%20Reference) (OtherBodyIndex :type Integer))
  (bind _door_track (Timeline|OpenDoorT Reverse)
    (:Update
      (Transformation|SetRelativeRotation (Variables|Default|GetDoorStaticMesh) (Math|Rotator|MakeRotator 0.0 0.0 (Math|Float|Lerp (Variables|Default|GetClosePosition) (Variables|Default|GetOpenPosition) _door_track)) false false))
    (:Finished
      (Variables|Default|SetisOpen? (not (Variables|Default|GetisOpen?))))))

(event Custom|OpenDoor
  (bind _door_track (Timeline|OpenDoorT Play)
    (:Update
      (Transformation|SetRelativeRotation (Variables|Default|GetDoorStaticMesh) (Math|Rotator|MakeRotator 0.0 0.0 (Math|Float|Lerp (Variables|Default|GetClosePosition) (Variables|Default|GetOpenPosition) _door_track)) false false))
    (:Finished
      (Variables|Default|SetisOpen? (not (Variables|Default|GetisOpen?))))))

(event Custom|CloseDoor
  (bind _door_track (Timeline|OpenDoorT Reverse)
    (:Update
      (Transformation|SetRelativeRotation (Variables|Default|GetDoorStaticMesh) (Math|Rotator|MakeRotator 0.0 0.0 (Math|Float|Lerp (Variables|Default|GetClosePosition) (Variables|Default|GetOpenPosition) _door_track)) false false))
    (:Finished
      (Variables|Default|SetisOpen? (not (Variables|Default|GetisOpen?))))))

(fn ConstructionScript)

(fn Interact
  (params (Interactor :type Character%20Object%20Reference))
  (bind _opendoort (Variables|Default|GetOpenDoorT))
  (if (not (Variables|Default|GetisOpen?))
    (Components|Timeline|SetPlayRate _opendoort (/ 1.0 (Variables|Default|GetOpenTime%28sec%29)))
    (CallFunction|OpenDoor)
    (else
      (Components|Timeline|SetPlayRate _opendoort (/ 1.0 (Variables|Default|GetCloseTime%28sec%29)))
      (CallFunction|CloseDoor))))